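; BP_PanelSwitch is a facility-device panel switch that shows its on/off state by rotating its mesh.
; SwitchChanged routes the On flag to OnTurnedOn or OnTurnedOff.
; Turning on adds 90 degrees to the mesh's current relative roll, while turning off sets roll to zero, both keeping pitch and yaw.
; The rotation is instant, with no animation or Tick logic.
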(event Custom|On%20Turned%20On
  (bind _mesh (Variables|Character|GetMesh))
  (bind _relativerotation (Variables|/Script/Engine.SceneComponent|GetRelativeRotation _mesh))
  (Transformation|SetRelativeRotation _mesh (Math|Rotator|MakeRotator (+ (.roll _relativerotation) 9e+01) (.pitch _relativerotation) (.yaw _relativerotation)) false false))

(event Custom|On%20Turned%20Off
  (bind _mesh (Variables|Character|GetMesh))
  (bind _relativerotation (Variables|/Script/Engine.SceneComponent|GetRelativeRotation _mesh))
  (Transformation|SetRelativeRotation _mesh (Math|Rotator|MakeRotator 0.0 (.pitch _relativerotation) (.yaw _relativerotation)) false false))

(event EventBeginPlay)

(event Collision|EventActorBeginOverlap
  (params (OtherActor :type Actor%20Object%20Reference)))

(event EventTick
  (params (DeltaSeconds :type Float%20%28single-precision%29)))

(event EventSwitchChanged
  (params (bOn :type Boolean) (bInstant :type Boolean))
  (if bOn
    (CallFunction|OnTurnedon)
    (else
      (CallFunction|OnTurnedOff))))

(fn ConstructionScript)